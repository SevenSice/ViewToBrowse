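; Actor component that moves its owning actor toward the location under the mouse when MousePressTeleport is triggered.
; The event stores the target from GetMouseUnderLocation and raises a Teleporting flag for a fixed Delay window.
; While the flag is set, Tick eases the owner toward the target with VInterpTo and unswept SetActorLocation, so the teleport is a smooth glide rather than an instant jump.
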(event Custom|MousePressTeleport
  (Variables|Default|SetTeleportLocation (CallFunction|GetMouseUnderLocation))
  (Variables|Default|SetTeleporting?? true)
  (Utilities|FlowControl|Delay 2.0)
  (Variables|Default|SetTeleporting?? false))

(event EventBeginPlay
  (Variables|Default|SetOwnerActor (Components|GetOwner)))

(event EventTick
  (params (DeltaSeconds :type Float%20%28single-precision%29))
  (if (Variables|Default|GetTeleporting??)
    (Transformation|SetActorLocation (Variables|Default|GetOwnerActor) (Math|Interpolation|VInterpTo (Transformation|GetActorLocation (Variables|Default|GetOwnerActor)) (Variables|Default|GetTeleportLocation) DeltaSeconds (Variables|Default|GetInterpSpeed)) false false)))