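; BP_MoveCharactor is a click-to-move actor that glides to the world location under the mouse.
; BeginPlay calls StartLocationDirection, and a left click stores the GetMouseUnderLocation result as the target, raising a Teleporting flag for a short delay.
; While flagged, Tick eases the actor toward the target with VInterpTo, without sweep, and interpolates the spring arm's pitch with FInterpTo.
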(event EventBeginPlay
  (CallFunction|StartLocationDirection))

(event EventTick
  (params (DeltaSeconds :type Float%20%28single-precision%29))
  (bind _springarm (Variables|Default|GetSpringArm))
  (bind _relativerotation (Variables|/Script/Engine.SceneComponent|GetRelativeRotation _springarm))
  (if (Variables|Default|GetTeleporting?)
    (Transformation|SetActorLocation (Math|Interpolation|VInterpTo (Transformation|GetActorLocation) (Variables|Default|GetTargetLocation) DeltaSeconds 3.0) false false)
    (Transformation|SetRelativeRotation _springarm (Math|Rotator|MakeRotator (.roll _relativerotation) (Math|Interpolation|FInterpTo (.pitch _relativerotation) 0.0 DeltaSeconds 3.0) (.yaw _relativerotation)) false false)))

(event Input|MouseEvents|LeftMouseButton
  (params (Key :type Key%20Structure))
  (:Pressed
    (Variables|Default|SetTeleporting? true)
    (Variables|Default|SetTargetLocation (.MouseToWorldLocation (CallFunction|GetMouseUnderLocation)))
    (Utilities|FlowControl|Delay 0.8)
    (Variables|Default|SetTeleporting? false)))

(fn ConstructionScript)