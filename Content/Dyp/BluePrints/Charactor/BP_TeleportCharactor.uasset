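; BP_TeleportCharactor is a character apparently meant to teleport between placed camera viewpoints, though that movement is unfinished.
; On BeginPlay it caches the location and rotation of each actor in CameraActorArray into target arrays.
; Tick checks a Teleporting flag but does nothing, and the Teleport call and LocationEnum switch are unconnected.
; TurnGraph maps axis inputs to controller yaw and pitch for looking around.
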(event EventTick
  (params (DeltaSeconds :type Float%20%28single-precision%29))
  (if (Variables|Default|Getteleporting?)
    _))

(event EventBeginPlay
  (for _array_element (Variables|目标点数组|GetCameraActorArray)
    (Utilities|Array|Add (Variables|目标点数组|GetTargetLocationArray) (Transformation|GetActorLocation _array_element))
    (Utilities|Array|Add (Variables|目标点数组|GetTargetRotationArray) (Transformation|GetActorRotation _array_element))))

(event Input|AxisEvents|InputAxisTurn_Pich
  (params (AxisValue :type Float%20%28single-precision%29))
  (Pawn|Input|AddControllerPitchInput AxisValue))

(event Input|AxisEvents|InputAxisTurn_Yaw
  (params (AxisValue :type Float%20%28single-precision%29))
  (Pawn|Input|AddControllerYawInput AxisValue))

(fn ConstructionScript)