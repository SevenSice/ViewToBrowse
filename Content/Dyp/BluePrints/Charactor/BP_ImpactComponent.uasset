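; BP_ImpactComponent tracks which BP_ImpactPoint actor is under the mouse cursor.
; Each tick it deprojects the mouse and line-traces on the Visibility channel, caching a hit point's location, rotation and reference and setting IsImpactActor.
; A miss clears only that flag, so the last point stays cached.
; Two helper functions switch that cached point's sphere collision between disabled and query-only.
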(event EventBeginPlay)

(event EventTick
  (params (DeltaSeconds :type Float%20%28single-precision%29))
  (bind (_worldlocation _worlddirection) (CallFunction|MousetoWorld))
  (bind _outhit (Collision|LineTraceByChannel _worldlocation (+ _worldlocation (* (Math|Vector|Normalize _worlddirection) 2e+04)) "TraceTypeQuery1" false 0 "None"))
  (bind _asbp_impact_point (Utilities|Casting|CastToBP_ImpactPoint (.HitActor (Collision|BreakHitResult _outhit)))
    (:then
      (Utilities|FlowControl|Sequence
        (:then_0
          (Variables|Default|SetImpactLocation (Transformation|GetActorLocation _asbp_impact_point))
          (Variables|Default|SetImpactRotation (Transformation|GetActorRotation _asbp_impact_point)))
        (:then_1
          (Variables|Default|SetIsImpactActor? true))
        (:then_2
          (Variables|Default|SetImpactActor _asbp_impact_point))))
    (:CastFailed
      (Variables|Default|SetIsImpactActor? false))))

(fn SetImpactActorNoCollision
  (bind _impactactor (Variables|Default|GetImpactActor))
  (Utilities|IsValid _impactactor
    (:Is%20Valid
      (Collision|SetCollisionEnabled (Variables|/Game/Dyp/BluePrints/UI/BP_ImpactPoint.BP_ImpactPoint_C|GetSphereCollision _impactactor) "NoCollision"))))

(fn SetImpactActorQueryCollision
  (bind _impactactor (Variables|Default|GetImpactActor))
  (Utilities|IsValid _impactactor
    (:Is%20Valid
      (Collision|SetCollisionEnabled (Variables|/Game/Dyp/BluePrints/UI/BP_ImpactPoint.BP_ImpactPoint_C|GetSphereCollision _impactactor) "QueryOnly"))))