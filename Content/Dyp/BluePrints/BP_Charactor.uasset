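; Player character for mouse-and-keyboard movement, with walk and fly modes and a laser pointer, apparently built for multiplayer.
; Holding left mouse spawns a camera-attached BP_LaserPointer, aimed each tick from the deprojected cursor through server-named events.
; Holding right mouse turns the view with screen-edge cursor wrapping, passing camera pitch to non-local copies.
; Flying disables capsule collision; returning to walking uses a floor trace and navmesh projection to avoid getting stuck.
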(event Custom|EventServerSendHitInformation
  (params (InVec :type Vector) (LaserIn :type BP%20Laser%20Pointer%20Object%20Reference) (Direction :type Vector))
  ;[1 1 1] 更新镭射光
  (Utilities|IsValid LaserIn
    (:Is%20Valid
      (Default|UpdateLaserPC LaserIn InVec Direction true))))

(event Custom|EventClientSendLaserInfos
  (bind _returnvalue (Game|GetPlayerController 0))
  (bind (_worldlocation _worlddirection) (Game|Player|ConvertMouseLocationToWorldSpace _returnvalue))
  ;[1 1 1] 更新镭射光
  (if (Pawn|IsLocallyControlled)
    (CallFunction|EventServerSendHitInformation _worldlocation (Variables|Default|GetCurrentLaserPointer) _worlddirection)))

(event EventTick
  (params (DeltaSeconds :type Float%20%28single-precision%29))
  (Utilities|FlowControl|Sequence
    (:then_0
      ;[1 1 1] 镭射
      (if (Variables|Default|GetLeftMouse)
        (Utilities|IsValid (Variables|Default|GetCurrentLaserPointer)
          (:Is%20Valid
            (CallFunction|EventClientSendLaserInfos)))))))

(event Custom|ServerEventLookUp
  (params (Target :type Scene%20Component%20Object%20Reference) (LookUp :type Float%20%28single-precision%29))
  ;[1 1 1] Look_角色抬头和转身
  (Transformation|SetRelativeRotation Target (Math|Rotator|MakeRotator 0.0 LookUp 0.0) false false)
  (CallFunction|EventSendClientRotation Target LookUp))

(event Custom|EventSendClientRotation
  (params (Target :type Scene%20Component%20Object%20Reference) (LookUp :type Float%20%28single-precision%29))
  ;[1 1 1] Look_角色抬头和转身
  (if (not (Pawn|IsLocallyControlled))
    (Transformation|SetRelativeRotation Target (Math|Rotator|MakeRotator 0.0 LookUp 0.0) false false)))

(event Custom|EventLeftClickToServer
  (params (SpawnTransformLocation :type Vector) (SpawnTransformRotation :type Rotator) (Pawn :type Pawn%20Object%20Reference))
  ;[1 1 1] 鼠标左键,发射光线
  (bind _returnvalue (Game|SpawnActorfromClass "/Game/Dyp/BluePrints/BP_LaserPointer.BP_LaserPointer_C" (Math|Transform|MakeTransform SpawnTransformLocation SpawnTransformRotation "1,1,1") "Undefined" self "0.000000,0.000000,0.000000" "0.000000,0.000000,0.000000" Pawn 0))
  (bind _output_get (Variables|Default|SetCurrentLaserPointer _returnvalue))
  (Transformation|AttachComponentToComponent _output_get (Variables|Default|GetCamera) "None" "SnapToTarget" "SnapToTarget" "KeepWorld" true)
  (Variables|Default|SetLeftMouse true))

(event Custom|EventEndLeftClickToServer
  (bind _currentlaserpointer (Variables|Default|GetCurrentLaserPointer))
  ;[1 1 1] 鼠标左键,发射光线
  (Variables|Default|SetLeftMouse false)
  (Utilities|IsValid _currentlaserpointer
    (:Is%20Valid
      (Default|UpdateLaserVR _currentlaserpointer "0, 0, 0" "0, 0, 0" false)
      (Actor|DestroyActor _currentlaserpointer))))

(event Custom|WrapMouseX
  (bind _returnvalue (Game|GetPlayerController 0))
  (bind _sizex (HUD|GetViewportSize _returnvalue))
  (bind (_locationx _locationy) (Game|Player|GetMousePosition _returnvalue))
  (bind _returnvalue_2 (Math|Float|Truncate _locationy))
  ;[1 1 1] Wrap mouse
  (if (<= _locationx 1e+01)
    (Class|PlayerController|SetMouseLocation (Game|GetPlayerController 0) (- _sizex 20) _returnvalue_2)
    (elif (>= _locationx (Math|Conversions|ToFloat(Integer) (- _sizex 10)))
      (Class|PlayerController|SetMouseLocation (Game|GetPlayerController 0) 20 _returnvalue_2))))

(event Custom|ToggleFlyModeServer
  (params (ApplyPulse :type Boolean))
  ;[1 1 1] move or Flying？
  (bind _isa (Utilities|FlowControl|FlipFlop)
    (:A
      (if (Class|NavMovementComponent|IsFlying (Variables|Character|GetCharacterMovement))
        _
        (elif ApplyPulse
          (Physics|AddImpulse (Variables|Character|GetCharacterMovement) "0, 0,700.000000" true)))
      (if _isa
        (CallFunction|EventChangeCollision "MOVE_Flying" "NoCollision")))
    (:B
      (CallFunction|EventChangeCollision "MOVE_Walking" "QueryAndPhysics"))))

(event Custom|WrapMouseY
  (bind _returnvalue (Game|GetPlayerController 0))
  (bind _sizey (HUD|GetViewportSize _returnvalue))
  (bind (_locationx _locationy) (Game|Player|GetMousePosition _returnvalue))
  (bind _returnvalue_2 (Math|Float|Truncate _locationx))
  ;[1 1 1] Wrap mouse
  (if (<= _locationy 1e+01)
    (Class|PlayerController|SetMouseLocation (Game|GetPlayerController 0) _returnvalue_2 (- _sizey 20))
    (elif (>= _locationy (Math|Conversions|ToFloat(Integer) (- _sizey 10)))
      (Class|PlayerController|SetMouseLocation (Game|GetPlayerController 0) _returnvalue_2 20))))

(event Custom|EventChangeCollision
  (params (NewMovementMode :type EMovementMode%20Enum :default "MOVE_None") (NewCollision :type ECollisionEnabled%20Enum :default "NoCollision"))
  (bind _returnvalue (Class|NavigationSystemV1|GetNavigationSystem))
  (bind _camera (Variables|Default|GetCamera))
  (bind _queryextent (Variables|Default|GetQueryExtent))
  (bind _camera_2 (Variables|Default|GetCamera))
  (bind _returnvalue_2 (Transformation|GetWorldLocation _camera))
  (bind _returnvalue_3 (Transformation|GetWorldLocation _camera_2))
  (bind _projectedlocation (AI|Navigation|ProjectPointtoNavigation _returnvalue _returnvalue_3 0 0 (Math|Vector|MakeVector _queryextent _queryextent _queryextent)))
  (Pawn|Components|CharacterMovement|SetMovementMode (Variables|Character|GetCharacterMovement) NewMovementMode 0)
  (Collision|SetCollisionEnabled (Variables|Collision|GetCapsuleComponent) NewCollision)
  ;[1 1 1] 在行走时找到一个有效位置，而不是卡在墙上
  (switch Utilities|FlowControl|Switch|SwitchonEMovementMode NewMovementMode
    (:MOVE_Walking
      ;;[1 1 1] 防止飞行切行走模式时卡在地板上，设置一个地板位置，走在地板上，而不是掉到下面的地板
      (bind _returnvalue_4 (Collision|LineTraceByChannel _returnvalue_2 (- _returnvalue_2 (Math|Vector|MakeVector 0.0 0.0 (+ (.z (Variables|/Script/Engine.SceneComponent|GetRelativeLocation _camera)) (Variables|/Script/Engine.CapsuleComponent|GetCapsuleHalfHeight (Variables|Collision|GetCapsuleComponent))))) "TraceTypeQuery1" false 0 "None"))
      (if _returnvalue_4
        (if (not (Math|Vector|Equal(Vector) _projectedlocation _returnvalue_3 5.0)) :!label _label
          (Transformation|SetActorLocation (+ _projectedlocation (Math|Vector|MakeVector 0.0 0.0 (Variables|/Script/Engine.CapsuleComponent|GetCapsuleHalfHeight (Variables|Collision|GetCapsuleComponent)))) false false))
        (else
          (Utilities|FlowControl|Delay 0.1)
          (if (not (AI|Components|NavMovement|IsFalling (Variables|Character|GetCharacterMovement)))
            (goto _label)))))))

(event Input|ActionEvents|InputActionToggleFlyMode
  (params (Key :type Key%20Structure))
  ;[1 1 1] move or Flying？
  (:Pressed
    (CallFunction|ToggleFlyModeServer true)))

(event Input|AxisEvents|InputAxisTurn_Pich
  (params (AxisValue :type Float%20%28single-precision%29))
  ;[1 1 1] Look_角色抬头和转身
  (if (Variables|Default|GetRightMouse)
    (CallFunction|WrapMouseX)
    (Pawn|Input|AddControllerPitchInput (* AxisValue (Variables|Default|GetLookSpeed) -1.0))
    (CallFunction|ServerEventLookUp (Variables|Default|GetCamera) (.pitch (Pawn|GetControlRotation :!class /Script/Engine.Pawn)))))

(event Input|AxisEvents|InputAxisMoveForward
  (params (AxisValue :type Float%20%28single-precision%29))
  (Pawn|Input|AddMovementInput (select (Class|NavMovementComponent|IsFlying (Variables|Character|GetCharacterMovement)) (Math|Vector|GetForwardVector (Pawn|GetControlRotation :!class /Script/Engine.Pawn)) (Math|Vector|GetForwardVector (Variables|Collision|GetCapsuleComponent))) (* AxisValue (Variables|Default|GetMoveSpeed)) false))

(event Input|AxisEvents|InputAxisMoveRight
  (params (AxisValue :type Float%20%28single-precision%29))
  (Pawn|Input|AddMovementInput (select (Class|NavMovementComponent|IsFlying (Variables|Character|GetCharacterMovement)) (Math|Vector|GetRightVector (Pawn|GetControlRotation :!class /Script/Engine.Pawn)) (Math|Vector|GetRightVector (Variables|Collision|GetCapsuleComponent))) (* AxisValue (Variables|Default|GetMoveSpeed)) false))

(event Input|AxisEvents|InputAxisMoveUp
  (params (AxisValue :type Float%20%28single-precision%29))
  ;[1 1 1] Fly Up/Down
  (if (Class|NavMovementComponent|IsFlying (Variables|Character|GetCharacterMovement))
    (Pawn|Input|AddMovementInput (Math|Vector|GetUpVector (Variables|Collision|GetCapsuleComponent)) (* AxisValue (Variables|Default|GetMoveSpeed)) false)))

(event Input|AxisEvents|InputAxisTurn_Yaw
  (params (AxisValue :type Float%20%28single-precision%29))
  ;[1 1 1] Look_角色抬头和转身
  (if (Variables|Default|GetRightMouse)
    (CallFunction|WrapMouseY)
    (Pawn|Input|AddControllerYawInput (* AxisValue (Variables|Default|GetLookSpeed)))))

(event Input|MouseEvents|LeftMouseButton
  (params (Key :type Key%20Structure))
  (bind _camera (Variables|Default|GetCamera))
  (bind _returnvalue (Transformation|GetWorldTransform _camera))
  ;[1 1 1] 鼠标左键,发射光线
  (:Pressed
    (if (not (Variables|Default|GetRightMouse))
      (CallFunction|EventLeftClicktoServer (.location _returnvalue) (.rotation _returnvalue) self)))
  (:Released
    (CallFunction|EventEndLeftClicktoServer)))

(event Input|MouseEvents|RightMouseButton
  (params (Key :type Key%20Structure))
  (bind _returnvalue (Game|GetPlayerController 0))
  (bind _returnvalue_2 (Game|GetPlayerController 0))
  (bind (_locationx _locationy) (Game|Player|GetMousePosition _returnvalue_2))
  ;[1 1 1] 鼠标右键
  (:Pressed
    (if (not (Variables|Default|GetLeftMouse))
      (Variables|Default|SetRightMouse true)
      (Variables|/Script/Engine.PlayerController|SetbShowMouseCursor _returnvalue_2 false)
      (Variables|Default|SetInitMousePosition (Math|Vector2D|MakeVector2D _locationx _locationy))))
  (:Released
    (if (Variables|Default|GetRightMouse)
      (Variables|Default|SetRightMouse false)
      (Class|PlayerController|SetMouseLocation _returnvalue (Math|Float|Truncate (.x (Variables|Default|GetInitMousePosition))) (Math|Float|Truncate (.y (Variables|Default|GetInitMousePosition))))
      (Variables|/Script/Engine.PlayerController|SetbShowMouseCursor _returnvalue true))))

(fn ConstructionScript)

(fn Arrived
  (return (Math|Vector|Equal(Vector) (Transformation|GetActorLocation) "0, 0, 0" 1.0)))

(fn GetMouseUnderLocation
  (bind _returnvalue (Game|GetPlayerController 0))
  (bind _hitresult (Game|Player|GetHitResultUnderCursorbyChannel _returnvalue "TraceTypeQuery1" true))
  (bind (_bblockinghit _binitialoverlap _time _distance _location _impactpoint _normal _impactnormal) (Collision|BreakHitResult _hitresult))
  (return (+ _location "0, 0,30.000000") (Math|Rotator|MakeRotationfromAxes _impactnormal "0, 0, 0" "0, 0, 0")))

(fn StartLocationDirection
  (bind _returnvalue (Transformation|GetActorLocation))
  (bind _returnvalue_2 (Transformation|GetActorRotation))
  (bind _scene (Variables|Default|GetScene))
  (bind _springarm (Variables|Default|GetSpringArm))
  (bind (_roll _pitch _yaw) (Math|Rotator|BreakRotator _returnvalue_2))
  (bind _relativerotation (Variables|/Script/Engine.SceneComponent|GetRelativeRotation _springarm))
  (bind _relativerotation_2 (Variables|/Script/Engine.SceneComponent|GetRelativeRotation _scene))
  (Transformation|SetActorLocation _returnvalue false true)
  (Transformation|SetRelativeRotation _springarm (Math|Rotator|MakeRotator (.roll _relativerotation) _pitch (.yaw _relativerotation)) false false)
  (Transformation|SetRelativeRotation _scene (Math|Rotator|MakeRotator (.roll _relativerotation_2) (.pitch _relativerotation_2) _yaw) false false)
  (return _returnvalue _returnvalue_2))