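; Blueprint function library of mouse helpers for player 0, plus a tick gating utility.
; MouseToWorld deprojects the cursor to a world position and direction, while GetMouseUnderLocation returns the Visibility hit under the cursor, raised slightly on Z.
; TickDoOnece cross-resets two DoOnce nodes to latch on changes in a boolean condition, but its first DoOnce drives no action.
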(fn MousetoWorld
  (bind _returnvalue (Game|GetPlayerController 0))
  (bind (_worldlocation _worlddirection _returnvalue_2) (Game|Player|ConvertMouseLocationToWorldSpace _returnvalue))
  (return _worldlocation _worlddirection _returnvalue_2))

(fn TickDoOnece
  (params (ExecutionCondition :type Boolean))
  (if ExecutionCondition
    (Utilities|FlowControl|Sequence
      (:then_0
        (Utilities|FlowControl|DoOnce false :!label _label))
      (:then_1
        (goto _label_2 Reset)))
    (else
      (Utilities|FlowControl|DoOnce false :!label _label_2
        (:Completed
          (goto _label Reset))))))

(fn GetMouseUnderLocation
  (return (+ (.Location (Collision|BreakHitResult (.HitResult (Game|Player|GetHitResultUnderCursorbyChannel (Game|GetPlayerController 0) "TraceTypeQuery1" false)))) "0, 0,30.000000")))