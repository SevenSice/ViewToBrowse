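; Free-flying camera pawn that starts at the StartCamera's transform and supports axis movement plus click-to-travel.
; Forward, right and up inputs move along the camera's axes and cancel any active travel.
; Left mouse release traces under the cursor and targets a point raised above the hit.
; Tick eases the pawn there with VInterpTo, leveling the camera to zero rotation via RInterpTo until arrival.
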(event EventBeginPlay
  ;[1 1 1] 初始化方向坐标
  (bind (_startlocation _startrotation) (CallFunction|StartLocationDirection))
  (Variables|Default|SetTargetLocation _startlocation)
  (Variables|Default|SetTargetRotation _startrotation))

(event EventTick
  (params (DeltaSeconds :type Float%20%28single-precision%29))
  ;[1 1 1] event tick
  (Utilities|FlowControl|Sequence
    (:then_0
      (if (Variables|Default|Getteleporting?)
        (Transformation|SetActorLocation (Math|Interpolation|VInterpTo (Transformation|GetActorLocation) (Variables|Default|GetTargetLocation) DeltaSeconds 5.0) false true)
        (if (not (CallFunction|Arrived))
          (Transformation|SetWorldRotation (Variables|Default|GetCamera) (Math|Interpolation|RInterpTo (Transformation|GetWorldRotation (Variables|Default|GetCamera)) (Variables|Default|GetTargetRotation) DeltaSeconds 5.0) false true))))))

(event Input|AxisEvents|InputAxisMoveForward
  (params (AxisValue :type Float%20%28single-precision%29))
  (Utilities|FlowControl|Sequence
    (:then_0
      (Pawn|Input|AddMovementInput (Math|Vector|GetForwardVector (Transformation|GetWorldRotation (Variables|Default|GetCamera))) AxisValue false))
    (:then_1
      (if (or (> AxisValue 0.0) (< AxisValue 0.0))
        (Variables|Default|Setteleporting? false)))))

(event Input|AxisEvents|InputAxisMoveRight
  (params (AxisValue :type Float%20%28single-precision%29))
  (Utilities|FlowControl|Sequence
    (:then_0
      (Pawn|Input|AddMovementInput (Math|Vector|GetRightVector (Transformation|GetWorldRotation (Variables|Default|GetCamera))) AxisValue false))
    (:then_1
      (if (or (> AxisValue 0.0) (< AxisValue 0.0))
        (Variables|Default|Setteleporting? false)))))

(event Input|AxisEvents|InputAxisMoveUp
  (params (AxisValue :type Float%20%28single-precision%29))
  (Utilities|FlowControl|Sequence
    (:then_0
      (Pawn|Input|AddMovementInput (Math|Vector|GetUpVector (Transformation|GetWorldRotation (Variables|Default|GetCamera))) AxisValue false))
    (:then_1
      (if (or (> AxisValue 0.0) (< AxisValue 0.0))
        (Variables|Default|Setteleporting? false)))))

(event Input|MouseEvents|LeftMouseButton
  (params (Key :type Key%20Structure))
  (:Released
    (Variables|Default|SetTargetLocation (.WorldLocation (CallFunction|GetMouseUnderlocation)))
    (Variables|Default|SetTargetRotation "0, 0, 0")
    (Variables|Default|Setteleporting? true)))

(event Input|KeyboardEvents|AnyKey
  (params (Key :type Key%20Structure))
  (:Pressed
    (if (Class|KismetInputLibrary|KeyIsKeyboardKey Key)
      _)))

(fn ConstructionScript)

(fn StartLocationDirection
  (bind _startcamera (Variables|Default|GetStartCamera))
  (bind _returnvalue (Transformation|GetActorLocation _startcamera))
  (bind _returnvalue_2 (Transformation|GetActorRotation _startcamera))
  (Transformation|Teleport _returnvalue _returnvalue_2)
  (Transformation|SetWorldRotation (Variables|Default|GetCamera) _returnvalue_2 false false)
  (return _returnvalue _returnvalue_2))

(fn GetMouseUnderlocation
  (bind _returnvalue (Game|GetPlayerController 0))
  (bind _hitresult (Game|Player|GetHitResultUnderCursorbyChannel _returnvalue "TraceTypeQuery1" true))
  (bind (_bblockinghit _binitialoverlap _time _distance _location _impactpoint _normal _impactnormal) (Collision|BreakHitResult _hitresult))
  (return (+ _location "0, 0,200.000000") (Math|Rotator|MakeRotationfromAxes _impactnormal "0, 0, 0" "0, 0, 0")))

(fn Arrived
  (return (Math|Vector|Equal(Vector) (Transformation|GetActorLocation) (Variables|Default|GetTargetLocation) 1.0)))